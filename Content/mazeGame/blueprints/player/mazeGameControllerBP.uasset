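; Player controller for the maze game that handles movement, sprint and mouse look for the mazeGamePawnBP pawn.
; BeginPlay caches the pawn, its start transform and the base move sensitivity, which sprint multiplies while held.
; Axis input moves the pawn directly in its local space without sweep, and mouse input sets its pitch and yaw.
; Jump and a wireframe helper mode exist only as comments.
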(event EventBeginPlay
  ;[1 1 1] Game start actions
  (Utilities|FlowControl|Sequence
    (:then_0
      (Utilities|ReferenceCast))
    (:then_1
      (Variables|Defaults|SetlevelStart (Transformation|GetActorTransform (Variables|Reference|GetplayerPawnRef)))
      (Variables|Defaults|SetmoveSensitivity (Variables|Defaults|GetbaseMovement)))
    (:then_2
      (Variables|Defaults|SetdisablePlayerInput false))))

(event EventTick
  (params (DeltaSeconds :type Float%20%28single-precision%29)))

(event Input|ActionEvents|InputActioninpSprint
  (params (Key :type Key%20Structure :default "None"))
  (bind _basemovement (Variables|Defaults|GetbaseMovement))
  ;[1 1 1] X Y movement
  (:Pressed
    (Variables|Defaults|SetmoveSensitivity (* _basemovement (Variables|Defaults|GetmovementMultiplier))))
  (:Released
    (Variables|Defaults|SetmoveSensitivity _basemovement)))

(event Input|ActionEvents|InputActioninpJump
  (params (Key :type Key%20Structure :default "None"))
  ;[1 1 1] Jump - write a macro
)

(event Input|ActionEvents|InputActioninpPrimaryFire
  (params (Key :type Key%20Structure :default "None"))
  ;[1 1 1] Helper mode - for now fire should make the level switch to wireframe whilst held
)

(event Input|AxisEvents|InputAxismoveForwards
  (params (AxisValue :type Float%20%28single-precision%29))
  ;[1 1 1] X Y movement
  (Utilities|BasicMovementControls AxisValue (stale Input|AxisEvents|InputAxismoveRight AxisValue)))

(event Input|AxisEvents|InputAxismoveRight
  (params (AxisValue :type Float%20%28single-precision%29))
  ;[1 1 1] X Y movement
  (Utilities|BasicMovementControls (stale Input|AxisEvents|InputAxismoveForwards AxisValue) AxisValue))

(event Input|MouseEvents|MouseY
  (params (AxisValue :type Float%20%28single-precision%29))
  (bind _playerpawnref (Variables|Reference|GetplayerPawnRef))
  (bind _mousesensitivity (Variables|Settings|GetmouseSensitivity))
  (bind _returnvalue (Transformation|GetActorRotation _playerpawnref))
  (bind (_roll _pitch _yaw) (Math|Rotator|BreakRotator _returnvalue))
  ;[1 1 1] Mouse look
  (Transformation|SetActorRotation _playerpawnref (Math|Rotator|MakeRotator _roll (+ (* AxisValue _mousesensitivity) _pitch) (+ _yaw (* _mousesensitivity (stale Input|MouseEvents|MouseX AxisValue))))))

(event Input|MouseEvents|MouseX
  (params (AxisValue :type Float%20%28single-precision%29))
  (bind _playerpawnref (Variables|Reference|GetplayerPawnRef))
  (bind _mousesensitivity (Variables|Settings|GetmouseSensitivity))
  (bind _returnvalue (Transformation|GetActorRotation _playerpawnref))
  (bind (_roll _pitch _yaw) (Math|Rotator|BreakRotator _returnvalue))
  ;[1 1 1] Mouse look
  (Transformation|SetActorRotation _playerpawnref (Math|Rotator|MakeRotator _roll (+ (* (stale Input|MouseEvents|MouseY AxisValue) _mousesensitivity) _pitch) (+ _yaw (* _mousesensitivity AxisValue)))))

(fn ConstructionScript)