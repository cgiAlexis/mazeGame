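; Game mode for the maze game that respawns the player's maze character after it is destroyed.
; On BeginPlay it casts the player character to MazeCharBP and binds a handler to its OnDestroyed event.
; The handler waits briefly, spawns a new character at the SpawnPoint transform and has the player controller possess it.
; It then calls Respawn to rebind the handler to the new character, so the cycle repeats.
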(event Custom|respawn
  ;[1 1 1] Event cast
  (bind _asmaze_char_bp (Utilities|Casting|CastTomazeCharBP (Game|GetPlayerCharacter 0)))
  ;[1 1 1] Respawn
  (Game|BindEventtoOnDestroyed _asmaze_char_bp (delegate Custom|eventDied)))

(event Custom|eventDied
  (params (DestroyedActor :type Actor%20Object%20Reference))
  ;[1 1 1] Respawn
  (Utilities|FlowControl|Delay 1.0)
  (bind _returnvalue (Game|SpawnActorfromClass "/Game/mazeGame/blueprints/mazeCharBP.mazeCharBP_C" (Variables|defaults|GetspawnPoint) "Undefined" 0 0))
  (Pawn|Possess (Game|GetPlayerController 0) _returnvalue)
  (CallFunction|Respawn))

(event EventBeginPlay
  (Utilities|FlowControl|Sequence
    (:then_0
      ;[1 1 1] Event cast
      (bind _asmaze_char_bp (Utilities|Casting|CastTomazeCharBP (Game|GetPlayerCharacter 0)))
      ;[1 1 1] Respawn
      (Game|BindEventtoOnDestroyed _asmaze_char_bp (delegate Custom|eventDied)))))

(event EventTick
  (params (DeltaSeconds :type Float%20%28single-precision%29)))

(fn ConstructionScript)